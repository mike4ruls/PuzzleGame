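; Collectible orb actor with a type (Nature, Desert, Volcanoe or Starter) that sets its sphere's material.
; Overlap events on its spheres detect the first-person character, cache its PlayerBP and toggle the character's widget.
; Tick reapplies the material when the type changes, otherwise polls for interaction while in range and not placed or picked up.
; Pickup adds the orb to the player's Orbs array and hides it rather than destroying it.
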(event OnComponentBeginOverlap(Sphere1)
  (params (OverlappedComponent :type Primitive%20Component%20Object%20Reference) (OtherActor :type Actor%20Object%20Reference) (OtherComp :type Primitive%20Component%20Object%20Reference) (OtherBodyIndex :type Integer) (bFromSweep :type Boolean) (SweepResult :type Hit%20Result%20Structure%20%28by%20ref%29))
  (bind _asfirst_person_character (Utilities|Casting|CastToFirstPersonCharacter OtherActor))
  (Variables|Default|SetInRange true)
  (Utilities|IsValid (Variables|Default|Getplayer)
    (:Is%20Valid
      _)
    (:Is%20Not%20Valid
      (Variables|Default|Setplayer (Variables|/Game/FirstPersonBP/Blueprints/FirstPersonCharacter.FirstPersonCharacter_C|GetplayerBP _asfirst_person_character))))
  (if (not (Variables|Default|GetPickedUp))
    (Rendering|SetVisibility (Variables|/Game/FirstPersonBP/Blueprints/FirstPersonCharacter.FirstPersonCharacter_C|GetWidget _asfirst_person_character) true false)))

(event OnComponentBeginOverlap(Sphere)
  (params (OverlappedComponent :type Primitive%20Component%20Object%20Reference) (OtherActor :type Actor%20Object%20Reference) (OtherComp :type Primitive%20Component%20Object%20Reference) (OtherBodyIndex :type Integer) (bFromSweep :type Boolean) (SweepResult :type Hit%20Result%20Structure%20%28by%20ref%29))
  (bind _asfirst_person_character (Utilities|Casting|CastToFirstPersonCharacter OtherActor))
  (Variables|Default|SetInRange true)
  (Utilities|IsValid (Variables|Default|Getplayer)
    (:Is%20Valid
      _)
    (:Is%20Not%20Valid
      (Variables|Default|Setplayer (Variables|/Game/FirstPersonBP/Blueprints/FirstPersonCharacter.FirstPersonCharacter_C|GetplayerBP _asfirst_person_character))))
  (if (not (Variables|Default|GetPickedUp))
    (Rendering|SetVisibility (Variables|/Game/FirstPersonBP/Blueprints/FirstPersonCharacter.FirstPersonCharacter_C|GetWidget (stale OnComponentBeginOverlap(Sphere1) _asfirst_person_character)) true false)))

(event OnComponentEndOverlap(Sphere1)
  (params (OverlappedComponent :type Primitive%20Component%20Object%20Reference) (OtherActor :type Actor%20Object%20Reference) (OtherComp :type Primitive%20Component%20Object%20Reference) (OtherBodyIndex :type Integer))
  (bind _asfirst_person_character (Utilities|Casting|CastToFirstPersonCharacter OtherActor))
  (Variables|Default|SetInRange false)
  (Rendering|SetVisibility (Variables|/Game/FirstPersonBP/Blueprints/FirstPersonCharacter.FirstPersonCharacter_C|GetWidget _asfirst_person_character) false false))

(event EventBeginPlay
  (CallFunction|SetMaterial))

(event Collision|EventActorBeginOverlap
  (params (OtherActor :type Actor%20Object%20Reference)))

(event EventTick
  (params (DeltaSeconds :type Float%20%28single-precision%29))
  (if (!= (Variables|Default|GetOrbType) (Variables|Default|GetPreviousOrbType))
    (CallFunction|SetMaterial)
    (elif (Math|Boolean|ANDBoolean (not (Variables|Default|GetPlacedDown)) (not (Variables|Default|GetPickedUp)) (Variables|Default|GetInRange))
      (if (Variables|/Game/Game/PlayerBP.PlayerBP_C|GetInteracting (Variables|Default|Getplayer))
        (CallFunction|PickUpOrb)))))

(fn ConstructionScript)

(fn SetMaterial
  (Rendering|Material|SetMaterial (Variables|Default|GetSphere) 0 (Utilities|Select :Index (Variables|Default|GetOrbType) :NewEnumerator0 "/Game/Game/Orb/Materials/NatureMat.NatureMat" :NewEnumerator1 "/Game/Game/Orb/Materials/DesertMat.DesertMat" :NewEnumerator2 "/Game/Game/Orb/Materials/VolcanoeMat.VolcanoeMat" :NewEnumerator3 "/Game/Game/Orb/Materials/StarterMat.StarterMat"))
  (Variables|Default|SetPreviousOrbType (Variables|Default|GetOrbType)))

(fn PickUpOrb
  (Utilities|Array|Add (Variables|/Game/Game/PlayerBP.PlayerBP_C|GetOrbs (Variables|Default|Getplayer)) self)
  (Rendering|SetVisibility (Variables|Default|GetDefaultSceneRoot) false true)
  (Variables|Default|SetPickedUp true))