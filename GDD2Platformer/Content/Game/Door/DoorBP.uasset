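; Door Blueprint that swings a pair of doors open and quits the game when the player enters its WaterWarp trigger.
; While OpenDoors is set, Tick calls RotateOpen to yaw LeftDoor and RightDoor in opposite directions at RotSpeed.
; Both calls add to one shared CurrentRot, so it advances twice per frame until reaching OpenDoorAngle sets RotDoorFinished.
; Overlap of WaterWarp by FirstPersonCharacter2 calls QuitGame.
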(event OnComponentBeginOverlap(waterWarp)
  (params (OverlappedComponent :type Primitive%20Component%20Object%20Reference) (OtherActor :type Actor%20Object%20Reference) (OtherComp :type Primitive%20Component%20Object%20Reference) (OtherBodyIndex :type Integer) (bFromSweep :type Boolean) (SweepResult :type Hit%20Result%20Structure%20%28by%20ref%29))
  (Utilities|Casting|CastToFirstPersonCharacter2 OtherActor)
  (Game|QuitGame 0 "Quit"))

(event EventBeginPlay)

(event Collision|EventActorBeginOverlap
  (params (OtherActor :type Actor%20Object%20Reference)))

(event EventTick
  (params (DeltaSeconds :type Float%20%28single-precision%29))
  (if (and (Variables|Default|GetOpenDoors) (not (Variables|Default|GetRotDoorFinished)))
    (CallFunction|RotateOpen DeltaSeconds (Variables|Default|GetLeftDoor) false)
    (bind _finished (CallFunction|RotateOpen DeltaSeconds (Variables|Default|GetRightDoor) true))
    (Variables|Default|SetRotDoorFinished _finished)))

(fn ConstructionScript)

(fn RotateOpen
  (params (deltaTime :type Float%20%28single-precision%29) (object :type Scene%20Component%20Object%20Reference) (RotateLeft :type Boolean))
  (bind _returnvalue (Transformation|GetWorldRotation object))
  (bind _returnvalue_2 (Transformation|GetWorldRotation object))
  (bind _rotspeed (Variables|Default|GetRotSpeed))
  (bind (_roll _pitch _yaw) (Math|Rotator|BreakRotator _returnvalue_2))
  (bind (_roll_2 _pitch_2 _yaw_2) (Math|Rotator|BreakRotator _returnvalue))
  (bind _returnvalue_3 (* deltaTime _rotspeed))
  (Variables|Default|SetcurrentRot (+ (Variables|Default|GetcurrentRot) _returnvalue_3))
  (if RotateLeft
    (Transformation|SetWorldRotation object (Math|Rotator|MakeRotator _roll _pitch (- _yaw _returnvalue_3)) false false)
    (else
      (Transformation|SetWorldRotation object (Math|Rotator|MakeRotator _roll_2 _pitch_2 (+ _yaw_2 _returnvalue_3)) false false)))
  (return (>= (Variables|Default|GetcurrentRot) (Variables|Default|GetOpenDoorAngle))))