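; Torch actor in the maze that the first-person character can pick up.
; Until held, it polls its Collider every tick for an overlapping character and checks that character's PlayerBP Interacting flag.
; On pickup it marks itself Held, zeroes its rotation, attaches to the character keeping world transform, and destroys the Collider.
; The location rotation uses a zero angle, so the torch effectively stays where it was.
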(event EventBeginPlay)

(event Collision|EventActorBeginOverlap
  (params (OtherActor :type Actor%20Object%20Reference)))

(event EventTick
  (params (DeltaSeconds :type Float%20%28single-precision%29))
  (bind _collider (Variables|Default|GetCollider))
  (bind _overlappingactors (Collision|GetOverlappingActors _collider "/Game/FirstPerson/Blueprints/FirstPersonCharacter.FirstPersonCharacter_C" :!class /Script/Engine.PrimitiveComponent))
  (bind _output (Utilities|Array|Get(acopy) _overlappingactors))
  (if (not (Variables|Default|GetHeld))
    (Utilities|IsValid _output
      (:Is%20Valid
        (bind _asfirst_person_character (Utilities|Casting|CastToFirstPersonCharacter _output))
        (if (Variables|/Game/Game/PlayerBP.PlayerBP_C|GetInteracting (Variables|/Game/FirstPerson/Blueprints/FirstPersonCharacter.FirstPersonCharacter_C|GetplayerBP _asfirst_person_character))
          (Variables|Default|SetHeld true)
          (Transformation|SetActorLocationAndRotation (Math|Vector|RotateVectorAroundAxis (Transformation|GetActorLocation) 0.0 (Transformation|GetActorLocation _asfirst_person_character)) "0.000000,0.000000,0.000000")
          (Transformation|AttachActorToActor _asfirst_person_character "None" "KeepWorld" "KeepWorld" "KeepWorld" false)
          (Components|DestroyComponent (Variables|Default|GetCollider)))))))

(fn ConstructionScript)