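; Maze arch actor with six plane panels, each configured by a type variable as Open, Wall or Vine.
; On BeginPlay, Open panels are destroyed, while the others get a stone wall or vine material to match their type.
; Each panel's hit event destroys it when it is a Vine and the FirstPersonCharacter hits it, so vines act as breakable passages while walls stay solid.
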(event OnComponentHit(Plane1)
  (params (HitComponent :type Primitive%20Component%20Object%20Reference) (OtherActor :type Actor%20Object%20Reference) (OtherComp :type Primitive%20Component%20Object%20Reference) (NormalImpulse :type Vector :default "0, 0, 0") (Hit :type Hit%20Result%20Structure%20%28by%20ref%29))
  (if (Utilities|Enum|Equal(Enum) (Variables|Default|GetPlane1_Type) "NewEnumerator2")
    (Utilities|Casting|CastToFirstPersonCharacter OtherActor)
    (Components|DestroyComponent (Variables|Default|GetPlane1))))

(event OnComponentHit(Plane3)
  (params (HitComponent :type Primitive%20Component%20Object%20Reference) (OtherActor :type Actor%20Object%20Reference) (OtherComp :type Primitive%20Component%20Object%20Reference) (NormalImpulse :type Vector :default "0, 0, 0") (Hit :type Hit%20Result%20Structure%20%28by%20ref%29))
  (if (Utilities|Enum|Equal(Enum) (Variables|Default|GetPlane3_Type) "NewEnumerator2")
    (Utilities|Casting|CastToFirstPersonCharacter OtherActor)
    (Components|DestroyComponent (Variables|Default|GetPlane3))))

(event OnComponentHit(Plane4)
  (params (HitComponent :type Primitive%20Component%20Object%20Reference) (OtherActor :type Actor%20Object%20Reference) (OtherComp :type Primitive%20Component%20Object%20Reference) (NormalImpulse :type Vector :default "0, 0, 0") (Hit :type Hit%20Result%20Structure%20%28by%20ref%29))
  (if (Utilities|Enum|Equal(Enum) (Variables|Default|GetPlane4_Type) "NewEnumerator2")
    (Utilities|Casting|CastToFirstPersonCharacter OtherActor)
    (Components|DestroyComponent (Variables|Default|GetPlane4))))

(event OnComponentHit(Plane5)
  (params (HitComponent :type Primitive%20Component%20Object%20Reference) (OtherActor :type Actor%20Object%20Reference) (OtherComp :type Primitive%20Component%20Object%20Reference) (NormalImpulse :type Vector :default "0, 0, 0") (Hit :type Hit%20Result%20Structure%20%28by%20ref%29))
  (if (Utilities|Enum|Equal(Enum) (Variables|Default|GetPlane5_Type) "NewEnumerator2")
    (Utilities|Casting|CastToFirstPersonCharacter OtherActor)
    (Components|DestroyComponent (Variables|Default|GetPlane5))))

(event OnComponentHit(Plane6)
  (params (HitComponent :type Primitive%20Component%20Object%20Reference) (OtherActor :type Actor%20Object%20Reference) (OtherComp :type Primitive%20Component%20Object%20Reference) (NormalImpulse :type Vector :default "0, 0, 0") (Hit :type Hit%20Result%20Structure%20%28by%20ref%29))
  (if (Utilities|Enum|Equal(Enum) (Variables|Default|GetPlane6_Type) "NewEnumerator2")
    (Utilities|Casting|CastToFirstPersonCharacter OtherActor)
    (Components|DestroyComponent (Variables|Default|GetPlane6))))

(event OnComponentHit(Plane2)
  (params (HitComponent :type Primitive%20Component%20Object%20Reference) (OtherActor :type Actor%20Object%20Reference) (OtherComp :type Primitive%20Component%20Object%20Reference) (NormalImpulse :type Vector :default "0, 0, 0") (Hit :type Hit%20Result%20Structure%20%28by%20ref%29))
  (if (Utilities|Enum|Equal(Enum) (Variables|Default|GetPlane2_Type) "NewEnumerator2")
    (Utilities|Casting|CastToFirstPersonCharacter OtherActor)
    (Components|DestroyComponent (Variables|Default|GetPlane2))))

(event EventBeginPlay
  (bind _plane1 (Variables|Default|GetPlane1))
  (bind _plane3 (Variables|Default|GetPlane3))
  (bind _plane3_type (Variables|Default|GetPlane3_Type))
  (bind _plane4 (Variables|Default|GetPlane4))
  (bind _plane4_type (Variables|Default|GetPlane4_Type))
  (bind _plane5_type (Variables|Default|GetPlane5_Type))
  (bind _plane5 (Variables|Default|GetPlane5))
  (bind _plane6_type (Variables|Default|GetPlane6_Type))
  (bind _plane6 (Variables|Default|GetPlane6))
  (bind _plane1_type (Variables|Default|GetPlane1_Type))
  (bind _plane2 (Variables|Default|GetPlane2))
  (bind _plane2_type (Variables|Default|GetPlane2_Type))
  (if (Utilities|Enum|Equal(Enum) _plane1_type "NewEnumerator0")
    (Components|DestroyComponent _plane1)
    (else
      (Rendering|Material|SetMaterial _plane1 0 (Utilities|Select :Index _plane1_type :NewEnumerator0 0 :NewEnumerator1 "/Game/FirstPerson/Textures/StoneWallMaterial.StoneWallMaterial" :NewEnumerator2 "/Game/FirstPerson/Textures/VineMaterial.VineMaterial"))))
  (if (Utilities|Enum|Equal(Enum) _plane2_type "NewEnumerator0")
    (Components|DestroyComponent _plane2)
    (else
      (Rendering|Material|SetMaterial _plane2 0 (Utilities|Select :Index _plane2_type :NewEnumerator0 0 :NewEnumerator1 "/Game/FirstPerson/Textures/StoneWallMaterial.StoneWallMaterial" :NewEnumerator2 "/Game/FirstPerson/Textures/VineMaterial.VineMaterial"))))
  (if (Utilities|Enum|Equal(Enum) _plane3_type "NewEnumerator0")
    (Components|DestroyComponent _plane3)
    (else
      (Rendering|Material|SetMaterial _plane3 0 (Utilities|Select :Index _plane3_type :NewEnumerator0 0 :NewEnumerator1 "/Game/FirstPerson/Textures/StoneWallMaterial.StoneWallMaterial" :NewEnumerator2 "/Game/FirstPerson/Textures/VineMaterial.VineMaterial"))))
  (if (Utilities|Enum|Equal(Enum) _plane4_type "NewEnumerator0")
    (Components|DestroyComponent _plane4)
    (else
      (Rendering|Material|SetMaterial _plane4 0 (Utilities|Select :Index _plane4_type :NewEnumerator0 0 :NewEnumerator1 "/Game/FirstPerson/Textures/StoneWallMaterial.StoneWallMaterial" :NewEnumerator2 "/Game/FirstPerson/Textures/VineMaterial.VineMaterial"))))
  (if (Utilities|Enum|Equal(Enum) _plane5_type "NewEnumerator0")
    (Components|DestroyComponent _plane5)
    (else
      (Rendering|Material|SetMaterial _plane5 0 (Utilities|Select :Index _plane5_type :NewEnumerator0 0 :NewEnumerator1 "/Game/FirstPerson/Textures/StoneWallMaterial.StoneWallMaterial" :NewEnumerator2 "/Game/FirstPerson/Textures/VineMaterial.VineMaterial"))))
  (if (Utilities|Enum|Equal(Enum) _plane6_type "NewEnumerator0")
    (Components|DestroyComponent _plane6)
    (else
      (Rendering|Material|SetMaterial _plane6 0 (Utilities|Select :Index _plane6_type :NewEnumerator0 0 :NewEnumerator1 "/Game/FirstPerson/Textures/StoneWallMaterial.StoneWallMaterial" :NewEnumerator2 "/Game/FirstPerson/Textures/VineMaterial.VineMaterial")))))

(event Collision|EventActorBeginOverlap
  (params (OtherActor :type Actor%20Object%20Reference)))

(event EventTick
  (params (DeltaSeconds :type Float%20%28single-precision%29)))

(fn ConstructionScript)