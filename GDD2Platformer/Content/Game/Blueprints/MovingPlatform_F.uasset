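; MovingPlatform_F is a moving platform Blueprint that slides its Cube component back and forth around its starting position.
; BeginPlay stores the cube's world location, then Tick offsets it by MoveSpeed scaled by delta time, without sweeping.
; MoveSpeed flips sign whenever the Y distance from the start is at or beyond a small hardcoded limit, with no clamping of the overshoot.
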(event EventBeginPlay
  (Variables|Default|SetstartLocation (Transformation|GetWorldLocation (Variables|Default|GetCube))))

(event Collision|EventActorBeginOverlap
  (params (OtherActor :type Actor%20Object%20Reference)))

(event EventTick
  (params (DeltaSeconds :type Float%20%28single-precision%29))
  (bind _cube (Variables|Default|GetCube))
  (bind _returnvalue (Transformation|GetWorldLocation _cube))
  (Transformation|SetWorldLocation _cube (+ (* (Variables|Default|GetmoveSpeed) DeltaSeconds) _returnvalue) false false)
  (if (>= (Math|Float|Absolute(Float) (- (.Y (Math|Vector|BreakVector _returnvalue)) (.Y (Math|Vector|BreakVector (Variables|Default|GetstartLocation))))) 2e+01)
    (Variables|Default|SetmoveSpeed (* (Variables|Default|GetmoveSpeed) -1.0))))

(fn ConstructionScript)