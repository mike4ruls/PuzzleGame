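; Rotating platform that, on R release, moves the level's Stairs actor to the mirrored position on its opposite side, without changing rotation.
; The interaction collider sets InRange, which is never cleared because end overlap also sets it true.
; IsActivePlatform compares the platform-to-stairs delta, within tolerance, against eight fixed axis-aligned diagonal offsets built by GetDirectionVector.
; A match activates the move and supplies the offset added to the platform's location.
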(event OnComponentBeginOverlap(InteractionCollider)
  (params (OverlappedComponent :type Primitive%20Component%20Object%20Reference) (OtherActor :type Actor%20Object%20Reference) (OtherComp :type Primitive%20Component%20Object%20Reference) (OtherBodyIndex :type Integer) (bFromSweep :type Boolean) (SweepResult :type Hit%20Result%20Structure%20%28by%20ref%29))
  (bind _asfirst_person_character (Utilities|Casting|CastToFirstPersonCharacter OtherActor))
  (Variables|Default|SetinRange true)
  (Utilities|IsValid (Variables|Default|GetPlayer)
    (:Is%20Not%20Valid
      (Variables|Default|SetPlayer _asfirst_person_character))))

(event OnComponentEndOverlap(InteractionCollider)
  (params (OverlappedComponent :type Primitive%20Component%20Object%20Reference) (OtherActor :type Actor%20Object%20Reference) (OtherComp :type Primitive%20Component%20Object%20Reference) (OtherBodyIndex :type Integer))
  (Variables|Default|SetinRange true))

(event EventBeginPlay
  (bind _outactors (Actor|GetAllActorsOfClass "/Game/Game/Blueprints/Stairs.Stairs_C"))
  (Variables|Default|SetStairs (Utilities|Array|Get(acopy) _outactors))
  (Input|EnableInput (Game|GetPlayerController 0)))

(event EventTick
  (params (DeltaSeconds :type Float%20%28single-precision%29)))

(event Input|KeyboardEvents|R
  (params (Key :type Key%20Structure :default "AnyKey"))
  (:Released
    (if (Variables|Default|GetinRange)
      (bind (_newstairposition _isactive) (CallFunction|IsActivePlatform))
      (if _isactive
        (Transformation|SetActorLocation (Variables|Default|GetStairs) (+ _newstairposition (Transformation|GetActorLocation)) false false)))))

(fn ConstructionScript
  (Variables|Default|SetzOffset 175.0)
  (Variables|Default|SetxyOffset 4.5e+02))

(fn GetDirectionVector
  (params (x :type Integer) (y :type Integer) (z :type Integer))
  (bind _zoffset (Variables|Default|GetzOffset))
  (bind _xyoffset (Variables|Default|GetxyOffset))
  (bind _returnvalue (* -1 _xyoffset))
  (bind _returnvalue_2 (Math|Float|MakeLiteralFloat _xyoffset))
  (bind _returnvalue_3 (Math|Float|MakeLiteralFloat _returnvalue))
  (return (Math|Vector|MakeVector (select (> x 0) _returnvalue_2 (select (< x 0) _returnvalue_3 0.0)) (select (> y 0) _returnvalue_2 (select (< y 0) _returnvalue_3 0.0)) (select (> z 0) (Math|Float|MakeLiteralFloat _zoffset) (select (< z 0) (Math|Float|MakeLiteralFloat (* -1 _zoffset)) 0.0)))))

(fn IsActivePlatform
  (bind _returnvalue (Transformation|GetActorLocation))
  (bind _stairs (Variables|Default|GetStairs))
  (bind _returnvalue_2 (Transformation|GetActorLocation _stairs))
  (bind _returnvalue_3 (- _returnvalue _returnvalue_2))
  (return (+ (select (Math|Vector|Equal(Vector) _returnvalue_3 (stale _direction) 5.0) (stale _direction) "") (select (Math|Vector|Equal(Vector) _returnvalue_3 (stale _direction) 5.0) (stale _direction) "") (select (Math|Vector|Equal(Vector) _returnvalue_3 (stale _direction) 5.0) (stale _direction) "") (select (Math|Vector|Equal(Vector) _returnvalue_3 (stale _direction) 5.0) (stale _direction) "") (select (Math|Vector|Equal(Vector) _returnvalue_3 (stale _direction) 5.0) (stale _direction) "") (select (Math|Vector|Equal(Vector) _returnvalue_3 (stale _direction) 5.0) (stale _direction) "") (select (Math|Vector|Equal(Vector) _returnvalue_3 (stale _direction) 5.0) (stale _direction) "") (select (Math|Vector|Equal(Vector) _returnvalue_3 (stale _direction) 5.0) (stale _direction) "")) (Math|Boolean|ORBoolean (Math|Vector|Equal(Vector) _returnvalue_3 (stale _direction) 5.0) (Math|Vector|Equal(Vector) _returnvalue_3 (stale _direction) 5.0) (Math|Vector|Equal(Vector) _returnvalue_3 (stale _direction) 5.0) (Math|Vector|Equal(Vector) _returnvalue_3 (stale _direction) 5.0) (Math|Vector|Equal(Vector) _returnvalue_3 (stale _direction) 5.0) (Math|Vector|Equal(Vector) _returnvalue_3 (stale _direction) 5.0) (Math|Vector|Equal(Vector) _returnvalue_3 (stale _direction) 5.0) (Math|Vector|Equal(Vector) _returnvalue_3 (stale _direction) 5.0))))