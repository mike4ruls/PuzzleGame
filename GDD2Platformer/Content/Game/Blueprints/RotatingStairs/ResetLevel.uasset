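; ResetLevel is an actor for the rotating stairs that decides whether a stairs reset is currently possible.
; On BeginPlay it gathers all RotatingPlatform actors and enables input from player controller 0.
; Each Tick it reads ResetStairs through the player character's PlayerBP, then sets ResetPossible true only if that flag is set and no platform reports InRange.
; The file computes this flag but contains no reset action.
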(event EventBeginPlay
  (bind _outactors (Actor|GetAllActorsOfClass "/Game/Game/Blueprints/RotatingStairs/RotatingPlatform.RotatingPlatform_C"))
  (Variables|Default|SetPlatforms _outactors)
  (Input|EnableInput (Game|GetPlayerController 0)))

(event EventTick
  (params (DeltaSeconds :type Float%20%28single-precision%29))
  (bind _asfirst_person_character_2 (Utilities|Casting|CastToFirstPersonCharacter2 (Variables|Default|GetPlayer)))
  (if (Variables|/Game/Game/PlayerBP.PlayerBP_C|GetResetStairs (Variables|/Game/FirstPersonBP/Blueprints/FirstPersonCharacter2.FirstPersonCharacter2_C|GetplayerBP _asfirst_person_character_2))
    (Variables|Default|SetCheck%20Reset%20Possible true)
    (for _array_element (Variables|Default|GetPlatforms)
      (bind _asrotating_platform (Utilities|Casting|CastToRotatingPlatform _array_element))
      (if (Variables|/Game/Game/Blueprints/RotatingStairs/RotatingPlatform.RotatingPlatform_C|GetinRange _asrotating_platform)
        (Variables|Default|SetCheck%20Reset%20Possible false)))
    (Variables|Default|SetReset%20Possible (Variables|Default|GetCheck%20Reset%20Possible))
    (else
      (Variables|Default|SetReset%20Possible false))))

(fn ConstructionScript)