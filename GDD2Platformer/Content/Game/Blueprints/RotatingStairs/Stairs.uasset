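; Stairs actor that snaps back to its starting transform when a level reset is flagged; it contains no rotation logic itself.
; BeginPlay caches the first-person player, enables input and records the initial transform.
; Tick polls every ResetLevel actor, and if any has ResetPossible set, restores that transform and clears the Resetting flag.
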(event EventBeginPlay
  (Utilities|FlowControl|Sequence
    (:then_0
      (bind _asfirst_person_character (Utilities|Casting|CastToFirstPersonCharacter (Game|GetPlayerCharacter 0)))
      (Utilities|IsValid (Variables|Default|GetPlayer)
        (:Is%20Not%20Valid
          (Variables|Default|SetPlayer _asfirst_person_character))))
    (:then_1
      (Input|EnableInput (Game|GetPlayerController 0))
      (Variables|Default|SetInitialTransform (Transformation|GetActorTransform)))))

(event EventTick
  (params (DeltaSeconds :type Float%20%28single-precision%29))
  (Utilities|FlowControl|Sequence
    (:then_0
      (bind _outactors (Actor|GetAllActorsOfClass "/Game/Game/Blueprints/RotatingStairs/ResetLevel.ResetLevel_C"))
      (for _array_element _outactors
        (bind _asreset_level (Utilities|Casting|CastToResetLevel _array_element))
        (if (or (Variables|/Game/Game/Blueprints/RotatingStairs/ResetLevel.ResetLevel_C|GetReset%20Possible _asreset_level) (Variables|Default|GetResetting))
          (Variables|Default|SetResetting true)
          (else
            (Variables|Default|SetResetting false)))))
    (:then_1
      (if (Variables|Default|GetResetting)
        (Transformation|SetActorTransform (Variables|Default|GetInitialTransform))
        (Variables|Default|SetResetting false)))))

(fn ConstructionScript)