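; Puzzle platform that a nearby first-person player turns left or right, or, with the invert action held, uses to roll adjoining stairs.
; Entering range attaches overlapping Stairs to four side boxes, and leaving detaches them.
; Tick polls player input flags, advances platform yaw or box roll, then snaps to degree steps tracked by rotation counters.
; Tick also polls ResetLevel actors to restore the initial transform, box rolls and counters.
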(event OnComponentBeginOverlap(InteractionCollider)
  (params (OverlappedComponent :type Primitive%20Component%20Object%20Reference) (OtherActor :type Actor%20Object%20Reference) (OtherComp :type Primitive%20Component%20Object%20Reference) (OtherBodyIndex :type Integer) (bFromSweep :type Boolean) (SweepResult :type Hit%20Result%20Structure%20%28by%20ref%29))
  (bind _asfirst_person_character (Utilities|Casting|CastToFirstPersonCharacter OtherActor))
  (Variables|Default|SetinRange true)
  (Utilities|IsValid (Variables|Default|GetPlayer)
    (:Is%20Valid
      _)
    (:Is%20Not%20Valid
      (Variables|Default|SetPlayer _asfirst_person_character)))
  (CallFunction|CheckforStairs))

(event EventBeginPlay
  (Input|EnableInput (Game|GetPlayerController 0))
  (Variables|Default|SetInitialTransform (Transformation|GetActorTransform)))

(event EventTick
  (params (DeltaSeconds :type Float%20%28single-precision%29))
  (bind _inrange (Variables|Default|GetinRange))
  (Utilities|FlowControl|Sequence
    (:then_0
      (bind _asfirst_person_character (Utilities|Casting|CastToFirstPersonCharacter (Variables|Default|GetPlayer)))
      (Utilities|FlowControl|Sequence
        (:then_0
          (bind _outactors (Actor|GetAllActorsOfClass "/Game/Game/Blueprints/RotatingStairs/ResetLevel.ResetLevel_C"))
          (for _array_element _outactors
            (bind _asreset_level (Utilities|Casting|CastToResetLevel _array_element))
            (CallFunction|IsLevelResetting _asreset_level)))
        (:then_1
          (if (Math|Boolean|ANDBoolean (Variables|/Game/Game/PlayerBP.PlayerBP_C|GetRotate%20Right (Variables|/Game/FirstPerson/Blueprints/FirstPersonCharacter.FirstPersonCharacter_C|GetplayerBP _asfirst_person_character)) (Variables|/Game/Game/PlayerBP.PlayerBP_C|GetInvertAction (Variables|/Game/FirstPerson/Blueprints/FirstPersonCharacter.FirstPersonCharacter_C|GetplayerBP _asfirst_person_character)) _inrange)
            (Variables|Default|SetRotating%20Stairs true)
            (Variables|Default|SetInvert%20Stair%20Rotation true)))
        (:then_2
          (if (Math|Boolean|ANDBoolean (Variables|/Game/Game/PlayerBP.PlayerBP_C|GetInvertAction (Variables|/Game/FirstPerson/Blueprints/FirstPersonCharacter.FirstPersonCharacter_C|GetplayerBP _asfirst_person_character)) (Variables|/Game/Game/PlayerBP.PlayerBP_C|GetRotate%20Left (Variables|/Game/FirstPerson/Blueprints/FirstPersonCharacter.FirstPersonCharacter_C|GetplayerBP _asfirst_person_character)) _inrange)
            (Variables|Default|SetRotating%20Stairs true)
            (Variables|Default|SetInvert%20Stair%20Rotation false)))
        (:then_3
          (if (Math|Boolean|ANDBoolean (Variables|/Game/Game/PlayerBP.PlayerBP_C|GetRotate%20Right (Variables|/Game/FirstPerson/Blueprints/FirstPersonCharacter.FirstPersonCharacter_C|GetplayerBP _asfirst_person_character)) (not (Variables|/Game/Game/PlayerBP.PlayerBP_C|GetInvertAction (Variables|/Game/FirstPerson/Blueprints/FirstPersonCharacter.FirstPersonCharacter_C|GetplayerBP _asfirst_person_character))) _inrange)
            (Variables|Default|SetRotating%20Platform true)
            (Variables|Default|SetInvert%20Platform%20Rotation false)))
        (:then_4
          (if (Math|Boolean|ANDBoolean (Variables|/Game/Game/PlayerBP.PlayerBP_C|GetRotate%20Left (Variables|/Game/FirstPerson/Blueprints/FirstPersonCharacter.FirstPersonCharacter_C|GetplayerBP _asfirst_person_character)) (not (Variables|/Game/Game/PlayerBP.PlayerBP_C|GetInvertAction (Variables|/Game/FirstPerson/Blueprints/FirstPersonCharacter.FirstPersonCharacter_C|GetplayerBP _asfirst_person_character))) _inrange)
            (Variables|Default|SetRotating%20Platform true)
            (Variables|Default|SetInvert%20Platform%20Rotation true)))))
    (:then_1
      (if (and (Variables|Default|GetRotating%20Stairs) (not (Variables|Default|GetResetting)))
        (bind _finished (CallFunction|RotateAllStairs DeltaSeconds))
        (if _finished
          (CallFunction|RoundAllStairs)
          (Variables|Default|SetRotating%20Stairs false)
          (if (Variables|Default|GetInvert%20Stair%20Rotation)
            (Math|Float|DecrementFloat (Variables|Default|GetstairRotNumber))
            (else
              (Math|Float|IncrementFloat (Variables|Default|GetstairRotNumber)))))))
    (:then_2
      (if (and (not (Variables|Default|GetResetting)) (Variables|Default|GetRotating%20Platform))
        (bind _donerotating (CallFunction|RotatePlatform DeltaSeconds))
        (if _donerotating
          (bind _returnvalue (CallFunction|RoundRotator (Transformation|GetActorRotation) false 0.0 false 0.0 true (Variables|Default|GetplatformRotateDegrees)))
          (Transformation|SetActorRotation _returnvalue)
          (Variables|Default|SetRotating%20Platform false)
          (if (Variables|Default|GetInvert%20Platform%20Rotation)
            (Math|Float|DecrementFloat (Variables|Default|GetplatformRotNumber))
            (else
              (Math|Float|IncrementFloat (Variables|Default|GetplatformRotNumber)))))))
    (:then_3
      (if (Variables|Default|GetResetting)
        (CallFunction|ResetSelf)
        (Variables|Default|SetResetting false)))))

(event Collision|EventActorEndOverlap
  (params (OtherActor :type Actor%20Object%20Reference))
  (Utilities|Casting|CastToFirstPersonCharacter OtherActor)
  (Variables|Default|SetinRange false)
  (CallFunction|DetatchAllStairs))

(fn ConstructionScript)

(fn CheckforStairs
  (CallFunction|AttachStairs (Variables|Default|GetFrontBox))
  (CallFunction|AttachStairs (Variables|Default|GetBackBox))
  (CallFunction|AttachStairs (Variables|Default|GetRightBox))
  (CallFunction|AttachStairs (Variables|Default|GetLeftBox)))

(fn AttachStairs
  (params (Collider :type Box%20Component%20Object%20Reference))
  (bind _array_element (Utilities|Array|ForEachLoopwithBreak (Collision|GetOverlappingActors Collider "/Game/Game/Blueprints/RotatingStairs/Stairs.Stairs_C" :!class /Script/Engine.PrimitiveComponent))
    (:LoopBody
      (Transformation|AttachComponentToComponent _array_element Collider "None" "KeepWorld" "KeepWorld" "KeepWorld" true))))

(fn RotateAllStairs
  (params (delta :type Float%20%28single-precision%29))
  (CallFunction|RotateStair (Variables|Default|GetFrontBox) delta)
  (CallFunction|RotateStair (Variables|Default|GetRightBox) delta)
  (CallFunction|RotateStair (Variables|Default|GetBackBox) delta)
  (CallFunction|RotateStair (Variables|Default|GetLeftBox) delta)
  (if (Variables|Default|GetInvert%20Stair%20Rotation)
    (return (< (Variables|Default|GetstairCurrentRot) (* (Variables|Default|GetstairRotNumber) (Variables|Default|GetstairRotateDegrees))))
    (else
      (return (> (Variables|Default|GetstairCurrentRot) (* (Variables|Default|GetstairRotNumber) (Variables|Default|GetstairRotateDegrees)))))))

(fn RotateStair
  (params (Collider :type Box%20Component%20Object%20Reference) (time :type Float%20%28single-precision%29))
  (bind _relativerotation (Variables|/Script/Engine.SceneComponent|GetRelativeRotation Collider))
  (bind (_roll _pitch _yaw) (Math|Rotator|BreakRotator _relativerotation))
  (if (Variables|Default|GetInvert%20Stair%20Rotation)
    (bind _output_get (Variables|Default|SetstairCurrentRot (- (Variables|Default|GetstairCurrentRot) (* time (Variables|Default|GetstairRotSpeed)))))
    (Transformation|SetRelativeRotation Collider (Math|Rotator|MakeRotator _output_get _pitch _yaw) false false)
    (else
      (bind _output_get_2 (Variables|Default|SetstairCurrentRot (+ (* time (Variables|Default|GetstairRotSpeed)) (Variables|Default|GetstairCurrentRot))))
      (Transformation|SetRelativeRotation Collider (Math|Rotator|MakeRotator _output_get_2 _pitch _yaw) false false))))

(fn RotatePlatform
  (params (Time :type Float%20%28single-precision%29))
  (bind _staticmeshcomponent (Variables|Debug|GetStaticMeshComponent))
  (bind _staticmeshcomponent_2 (Variables|Debug|GetStaticMeshComponent))
  (bind _relativerotation (Variables|/Script/Engine.SceneComponent|GetRelativeRotation _staticmeshcomponent))
  (bind (_roll _pitch) (Math|Rotator|BreakRotator _relativerotation))
  (if (Variables|Default|GetInvert%20Platform%20Rotation)
    (bind _output_get (Variables|Default|SetplatformCurrentRot (- (Variables|Default|GetplatformCurrentRot) (* (Variables|Default|GetplatformRotSpeed) Time))))
    (Transformation|SetRelativeRotation _staticmeshcomponent_2 (Math|Rotator|MakeRotator _roll _pitch _output_get) false false)
    (return (< (Variables|Default|GetplatformCurrentRot) (* (Variables|Default|GetplatformRotNumber) (Variables|Default|GetplatformRotateDegrees))))
    (else
      (bind _output_get_2 (Variables|Default|SetplatformCurrentRot (+ (* Time (Variables|Default|GetplatformRotSpeed)) (Variables|Default|GetplatformCurrentRot))))
      (Transformation|SetRelativeRotation _staticmeshcomponent_2 (Math|Rotator|MakeRotator _roll _pitch _output_get_2) false false)
      (return (> (Variables|Default|GetplatformCurrentRot) (* (Variables|Default|GetplatformRotNumber) (Variables|Default|GetplatformRotateDegrees)))))))

(fn IsLevelResetting
  (params (Reset%20Level%20BP :type Reset%20Level%20Object%20Reference))
  (if (or (Variables|/Game/Game/Blueprints/RotatingStairs/ResetLevel.ResetLevel_C|GetReset%20Possible Reset%20Level%20BP) (Variables|Default|GetResetting))
    (Variables|Default|SetResetting true)
    (else
      (Variables|Default|SetResetting false))))

(fn ResetSelf
  (Utilities|FlowControl|Sequence
    (:then_0
      (Variables|Default|SetstairRotNumber 1.0)
      (Variables|Default|SetplatformRotNumber 1.0)
      (Variables|Default|SetstairCurrentRot 0.0)
      (Variables|Default|SetplatformCurrentRot 0.0))
    (:then_1
      (CallFunction|ResetRotator (Variables|Default|GetFrontBox))
      (CallFunction|ResetRotator (Variables|Default|GetRightBox))
      (CallFunction|ResetRotator (Variables|Default|GetBackBox))
      (CallFunction|ResetRotator (Variables|Default|GetLeftBox)))
    (:then_2
      (Transformation|SetActorTransform (Variables|Default|GetInitialTransform))
      (Variables|Default|SetResetting false))))

(fn ResetRotator
  (params (Collider :type Box%20Component%20Object%20Reference))
  (bind _relativerotation (Variables|/Script/Engine.SceneComponent|GetRelativeRotation Collider))
  (bind (_roll _pitch _yaw) (Math|Rotator|BreakRotator _relativerotation))
  (Transformation|SetRelativeRotation Collider (Math|Rotator|MakeRotator (Variables|Default|GetstairCurrentRot) _pitch _yaw) false false))

(fn DetatchAllStairs
  (CallFunction|DetatchStair (Variables|Default|GetFrontBox))
  (CallFunction|DetatchStair (Variables|Default|GetRightBox))
  (CallFunction|DetatchStair (Variables|Default|GetBackBox))
  (CallFunction|DetatchStair (Variables|Default|GetLeftBox)))

(fn DetatchStair
  (params (Collider :type Box%20Component%20Object%20Reference))
  (bind _array_element (Utilities|Array|ForEachLoopwithBreak (Collision|GetOverlappingActors Collider "/Game/Game/Blueprints/RotatingStairs/Stairs.Stairs_C" :!class /Script/Engine.PrimitiveComponent))
    (:LoopBody
      (Transformation|DetachFromActor _array_element "KeepWorld" "KeepWorld" "KeepWorld"))))

(fn RoundRotator
  (params (Unrounded%20Rotator :type Rotator) (roundX :type Boolean) (Round%20To%20Nearest%20X :type Float%20%28single-precision%29) (roundY :type Boolean) (Round%20To%20Nearest%20Y :type Float%20%28single-precision%29) (roundZ :type Boolean) (Round%20To%20Nearest%20Z :type Float%20%28single-precision%29))
  (bind (_roll _pitch _yaw) (Math|Rotator|BreakRotator Unrounded%20Rotator))
  (bind (_roll_2 _pitch_2 _yaw_2) (Math|Rotator|BreakRotator Unrounded%20Rotator))
  (bind (_roll_3 _pitch_3 _yaw_3) (Math|Rotator|BreakRotator Unrounded%20Rotator))
  (if roundX
    (bind _returnvalue (CallFunction|RoundtoNearest _roll_3 Round%20To%20Nearest%20X))
    (if roundY
      (bind _returnvalue_2 (CallFunction|RoundtoNearest (.Pitch (Math|Rotator|BreakRotator (Math|Rotator|MakeRotator _returnvalue _pitch_3 _yaw_3))) Round%20To%20Nearest%20Y))
      (if roundZ
        (bind _returnvalue_3 (CallFunction|RoundtoNearest (.Yaw (Math|Rotator|BreakRotator (Math|Rotator|MakeRotator (.Roll (Math|Rotator|BreakRotator (Math|Rotator|MakeRotator _returnvalue _pitch_3 _yaw_3))) _returnvalue_2 (.Yaw (Math|Rotator|BreakRotator (Math|Rotator|MakeRotator _returnvalue _pitch_3 _yaw_3)))))) Round%20To%20Nearest%20Z))
        (return (Math|Rotator|MakeRotator (.Roll (Math|Rotator|BreakRotator (Math|Rotator|MakeRotator (.Roll (Math|Rotator|BreakRotator (Math|Rotator|MakeRotator _returnvalue _pitch_3 _yaw_3))) _returnvalue_2 (.Yaw (Math|Rotator|BreakRotator (Math|Rotator|MakeRotator _returnvalue _pitch_3 _yaw_3)))))) (.Pitch (Math|Rotator|BreakRotator (Math|Rotator|MakeRotator (.Roll (Math|Rotator|BreakRotator (Math|Rotator|MakeRotator _returnvalue _pitch_3 _yaw_3))) _returnvalue_2 (.Yaw (Math|Rotator|BreakRotator (Math|Rotator|MakeRotator _returnvalue _pitch_3 _yaw_3)))))) _returnvalue_3)) ; Round to X, Y, and Z
        (else
          (return (Math|Rotator|MakeRotator (.Roll (Math|Rotator|BreakRotator (Math|Rotator|MakeRotator _returnvalue _pitch_3 _yaw_3))) _returnvalue_2 (.Yaw (Math|Rotator|BreakRotator (Math|Rotator|MakeRotator _returnvalue _pitch_3 _yaw_3))))) ; Round to X and Y
        ))
      (elif roundZ
        (bind _returnvalue_4 (CallFunction|RoundtoNearest (.Yaw (Math|Rotator|BreakRotator (Math|Rotator|MakeRotator _returnvalue _pitch_3 _yaw_3))) Round%20To%20Nearest%20Z))
        (return (Math|Rotator|MakeRotator (.Roll (Math|Rotator|BreakRotator (Math|Rotator|MakeRotator _returnvalue _pitch_3 _yaw_3))) (.Pitch (Math|Rotator|BreakRotator (Math|Rotator|MakeRotator _returnvalue _pitch_3 _yaw_3))) _returnvalue_4)) ; Round X and Z
        (else
          (return (Math|Rotator|MakeRotator _returnvalue _pitch_3 _yaw_3)) ; Only round X
        )))
    (elif roundY
      (bind _returnvalue_5 (CallFunction|RoundtoNearest _pitch Round%20To%20Nearest%20Y))
      (if roundZ
        (bind _returnvalue_6 (CallFunction|RoundtoNearest (.Yaw (Math|Rotator|BreakRotator (Math|Rotator|MakeRotator _roll _returnvalue_5 _yaw))) Round%20To%20Nearest%20Z))
        (return (Math|Rotator|MakeRotator (.Roll (Math|Rotator|BreakRotator (Math|Rotator|MakeRotator _roll _returnvalue_5 _yaw))) (.Pitch (Math|Rotator|BreakRotator (Math|Rotator|MakeRotator _roll _returnvalue_5 _yaw))) _returnvalue_6)) ; Round Y and Z
        (else
          (return (Math|Rotator|MakeRotator _roll _returnvalue_5 _yaw)) ; Only round Y
        ))
      (elif roundZ
        (bind _returnvalue_7 (CallFunction|RoundtoNearest _yaw_2 Round%20To%20Nearest%20Z))
        (return (Math|Rotator|MakeRotator _roll_2 _pitch_2 _returnvalue_7)) ; Only round Z
        (else
          (return Unrounded%20Rotator) ; Don't round
        )))))

(fn RoundtoNearest
  (params (Unrounded%20Number :type Float%20%28single-precision%29) (Round%20To%20nearest :type Float%20%28single-precision%29))
  (return (* (Math|Float|Round (/ Unrounded%20Number Round%20To%20nearest)) Round%20To%20nearest)))

(fn RoundAllStairs
  (Utilities|FlowControl|Sequence
    (:then_0
      (bind _returnvalue (CallFunction|RoundRotator (Variables|/Script/Engine.SceneComponent|GetRelativeRotation (Variables|Default|GetFrontBox)) true (Variables|Default|GetstairRotateDegrees) false 0.0 false 0.0))
      (Transformation|SetRelativeRotation (Variables|Default|GetFrontBox) _returnvalue false false))
    (:then_1
      (bind _returnvalue_2 (CallFunction|RoundRotator (Variables|/Script/Engine.SceneComponent|GetRelativeRotation (Variables|Default|GetRightBox)) true (Variables|Default|GetstairRotateDegrees) false 0.0 false 0.0))
      (Transformation|SetRelativeRotation (Variables|Default|GetRightBox) _returnvalue_2 false false))
    (:then_2
      (bind _returnvalue_3 (CallFunction|RoundRotator (Variables|/Script/Engine.SceneComponent|GetRelativeRotation (Variables|Default|GetBackBox)) true (Variables|Default|GetstairRotateDegrees) false 0.0 false 0.0))
      (Transformation|SetRelativeRotation (Variables|Default|GetBackBox) _returnvalue_3 false false))
    (:then_3
      (bind _returnvalue_4 (CallFunction|RoundRotator (Variables|/Script/Engine.SceneComponent|GetRelativeRotation (Variables|Default|GetLeftBox)) true (Variables|Default|GetstairRotateDegrees) false 0.0 false 0.0))
      (Transformation|SetRelativeRotation (Variables|Default|GetLeftBox) _returnvalue_4 false false))))