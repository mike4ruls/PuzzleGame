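; Pressure plate tile for a memory-style path puzzle, where the player must step on safe tiles in numbered order.
; On first hit it sinks on a looping timer and turns green, advancing the player's tile counter, or red, flagging the player dead.
; StartingDisplay previews it in green until a countdown restores the base material.
; BeginPlay also moves the Sphere component to one of four random spawn points.
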(event EventBeginPlay
  (Variables|Default|SetmoveDownFinalHieght (- (.Z (Math|Vector|BreakVector (Transformation|GetWorldLocation (Variables|Default|GetPlate)))) (Variables|Default|GetmoveDownHeight)))
  (CallFunction|LoadSpawnPoints)
  (CallFunction|ChoseSpawn))

(event Collision|EventActorBeginOverlap
  (params (OtherActor :type Actor%20Object%20Reference)))

(event Collision|EventHit
  (params (MyComp :type Primitive%20Component%20Object%20Reference) (Other :type Actor%20Object%20Reference) (OtherComp :type Primitive%20Component%20Object%20Reference) (bSelfMoved :type Boolean) (HitLocation :type Vector :default "0, 0, 0") (HitNormal :type Vector :default "0, 0, 0") (NormalImpulse :type Vector :default "0, 0, 0") (Hit :type Hit%20Result%20Structure%20%28by%20ref%29))
  (bind _asfirst_person_character (Utilities|Casting|CastToFirstPersonCharacter Other))
  (Utilities|IsValid (Variables|Default|Getplayer)
    (:Is%20Valid
      _)
    (:Is%20Not%20Valid
      (Variables|Default|Setplayer _asfirst_person_character)))
  (if (Variables|Default|GetIsPressed)
    _
    (else
      (CallFunction|TurnonPlate)))
  (Variables|Default|SetIsPressed true))

(event EventTick
  (params (DeltaSeconds :type Float%20%28single-precision%29)))

(fn ConstructionScript)

(fn StartingDisplay
  (Rendering|Material|SetMaterial (Variables|Default|GetPlate) 0 "/Game/Game/Materials/GreenMat.GreenMat")
  (Utilities|Time|SetTimerbyFunctionName self "TurnOffCountDown" 1.0 true))

(fn TurnOffCountDown
  (bind _result (Math|Float|DecrementFloat (Variables|Default|GetcountdownTime))
    (:%20%20
      (if (<= _result 0.0)
        (if (not (Variables|Default|GetIsPressed))
          (Rendering|Material|SetMaterial (Variables|Default|GetPlate) 0 "/Game/FirstPerson/Meshes/BaseMaterial.BaseMaterial"))
        (Class|KismetSystemLibrary|PauseTimer self "TurnOffCountDown")))))

(fn TurnonPlate
  (Utilities|Time|SetTimerbyFunctionName self "MoveDown" 0.01 true)
  (if (and (Variables|Default|GetIsSafe) (== (Variables|Default|GetTileNum) (Variables|/Game/Game/PlayerBP.PlayerBP_C|GetcurrentTileNum (Variables|/Game/FirstPerson/Blueprints/FirstPersonCharacter.FirstPersonCharacter_C|GetplayerBP (Variables|Default|Getplayer)))))
    (Rendering|Material|SetMaterial (Variables|Default|GetPlate) 0 "/Game/Game/Materials/GreenMat.GreenMat")
    (Math|Integer|IncrementInt (Variables|/Game/Game/PlayerBP.PlayerBP_C|GetcurrentTileNum (Variables|/Game/FirstPerson/Blueprints/FirstPersonCharacter.FirstPersonCharacter_C|GetplayerBP (Variables|Default|Getplayer))))
    (else
      (Rendering|Material|SetMaterial (Variables|Default|GetPlate) 0 "/Game/Game/Materials/RedMat.RedMat")
      (Variables|/Game/Game/PlayerBP.PlayerBP_C|SetDed (Variables|/Game/FirstPerson/Blueprints/FirstPersonCharacter.FirstPersonCharacter_C|GetplayerBP (Variables|Default|Getplayer)) true))))

(fn MoveDown
  (bind _returnvalue (Utilities|Time|GetWorldDeltaSeconds))
  (bind _movedownspeed (Variables|Default|GetmoveDownSpeed))
  (bind _plate (Variables|Default|GetPlate))
  (bind _returnvalue_2 (Transformation|GetWorldLocation _plate))
  (bind _returnvalue_3 (* _movedownspeed _returnvalue))
  (bind (_x _y _z) (Math|Vector|BreakVector _returnvalue_2))
  (bind _returnvalue_4 (- _z _returnvalue_3))
  (Transformation|SetWorldLocation _plate (Math|Vector|MakeVector _x _y _returnvalue_4) false false)
  (if (<= _returnvalue_4 (Variables|Default|GetmoveDownFinalHieght))
    (Class|KismetSystemLibrary|PauseTimer self "MoveDown")))

(fn LoadSpawnPoints
  (Utilities|Array|Add (Variables|Default|GetspawnPpoints) (Variables|Default|GetSpawnPoint1))
  (Utilities|Array|Add (Variables|Default|GetspawnPpoints) (Variables|Default|GetSpawnPoint2))
  (Utilities|Array|Add (Variables|Default|GetspawnPpoints) (Variables|Default|GetSpawnPoint3))
  (Utilities|Array|Add (Variables|Default|GetspawnPpoints) (Variables|Default|GetSpawnPoint4)))

(fn ChoseSpawn
  (bind _spawnppoints (Variables|Default|GetspawnPpoints))
  (Transformation|SetRelativeLocation (Variables|Default|GetSphere) (Variables|/Script/Engine.SceneComponent|GetRelativeLocation (Utilities|Array|Get(acopy) _spawnppoints (Math|Random|RandomIntegerinRange 0 (- (Utilities|Array|Length _spawnppoints) 1)))) false false))