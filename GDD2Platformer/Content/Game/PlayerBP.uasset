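; PlayerBP is a player Blueprint that turns held keys into state flags for interacting, rotating, resetting stairs and inverting an action.
; It enables input from the first player controller on BeginPlay, then each key press sets a boolean and its release clears it.
; The Blueprint only records these flags and never reads them, and its Tick and construction script are empty.
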(event EventBeginPlay
  (Input|EnableInput (Game|GetPlayerController 0)))

(event EventTick
  (params (DeltaSeconds :type Float%20%28single-precision%29)))

(event Input|KeyboardEvents|E
  (params (Key :type Key%20Structure))
  (:Pressed
    (Variables|Default|SetInteracting true))
  (:Released
    (Variables|Default|SetInteracting false)))

(event Input|KeyboardEvents|LeftShift
  (params (Key :type Key%20Structure))
  (:Pressed
    (Variables|Default|SetInvertAction true))
  (:Released
    (Variables|Default|SetInvertAction false)))

(event Input|KeyboardEvents|R
  (params (Key :type Key%20Structure))
  (:Pressed
    (Variables|Default|SetRotating true))
  (:Released
    (Variables|Default|SetRotating false)))

(event Input|KeyboardEvents|Z
  (params (Key :type Key%20Structure))
  (:Pressed
    (Variables|Default|SetResetStairs true))
  (:Released
    (Variables|Default|SetResetStairs false)))

(fn ConstructionScript)